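; Base physics actor that a character can look at, pick up and drop, notifying that character through interface messages.
; Look-at toggles a widget labeled with a name trimmed from the class name, plus a timer for a blinking debug-sphere highlight.
; Pickup lerps the actor by timeline to a bounds-scaled point ahead of player 0, then disables physics and follows that point on Tick.
; Drop re-enables physics.
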(event `LookAtInterface.OnPickup`
  (params (InInstigator :type "Actor Object Reference"))
  (bind (_outtransf_location _outtransf_rotation) (`KismetMathLibrary.BreakTransform` (`self.GetTargetTransform`)))
  (bind _output_get (set `self.PickupCharacter` InInstigator))
  (if (`KismetSystemLibrary.DoesImplementInterface` _output_get "/Script/PhysicsAudio.LookAtInterface")
    (if (`self.bCanBePickedUp`)
      (set `self.InitTransf` (`self.GetTransform`))
      (set `self.FinishTransf` (`self.GetTransform` (`self.PickupCharacter`)))
      (bind (_direction _lerp) (`Timeline|Timeline_0` :!via `PlayFromStart`)
        (:`Update`
          (set `self.FinishTransf` (`KismetMathLibrary.MakeTransform` _outtransf_location _outtransf_rotation))
          (`self.K2_SetActorTransform` (`KismetMathLibrary.TLerp` (`self.InitTransf`) (`self.FinishTransf`) _lerp)))
        (:`Finished`
          (set `self.bPickedUp` true)
          (`PrimitiveComponent.SetSimulatePhysics` (`self.StaticMeshComponent`) false)
          (message `LookAtInterface.OnPickup` (`self.PickupCharacter`) self))))))

(event `LookAtInterface.OnDrop`
  (params (InInstigator :type "Actor Object Reference"))
  (bind _output_get (set `self.PickupCharacter` InInstigator))
  (if (`KismetSystemLibrary.DoesImplementInterface` _output_get "/Script/PhysicsAudio.LookAtInterface")
    (if (`self.bCanBePickedUp`)
      (set `self.bPickedUp` false)
      (`PrimitiveComponent.SetSimulatePhysics` (`self.StaticMeshComponent`) true)
      (message `LookAtInterface.OnDrop` (`self.PickupCharacter`) self))))

(event `self.ReceiveBeginPlay`
  (`self.UpdateWidgetText`))

(event `LookAtInterface.OnLookAtStarted`
  (bind _lookattimer (`self.LookAtTimer`))
  (set `self.bLookedAt` true)
  (`SceneComponent.SetVisibility` (`self.WidgetComponent`) (`self.bLookedAt`) false :!label _label)
  (if (`self.bCanBePickedUp`)
    (if (`self.bLookedAt`)
      (`KismetSystemLibrary.K2_ClearAndInvalidateTimerHandle` _lookattimer)
      (bind _returnvalue (`KismetSystemLibrary.K2_SetTimerDelegate` (`|CreateDelegate` :!event `Blink`) 0.5 true))
      (set `self.LookAtTimer` _returnvalue)
      (else
        (`KismetSystemLibrary.K2_ClearAndInvalidateTimerHandle` _lookattimer)))))

(event `self.UpdateWidgetText`
  (bind _aswbp_look_at_widget (cast `/Game/UI/WBP_LookAtWidget` (`WidgetComponent.GetWidget` (`self.WidgetComponent`))))
  (set `/Game/UI/WBP_LookAtWidget.ActorName` (`self.ItemName`) _aswbp_look_at_widget))

(event `LookAtInterface.OnLookAtFinished`
  (set `self.bLookedAt` false)
  (goto _label))

(event `Blink`
  (if (and (not (`self.bPickedUp`)) (`self.bLookedAt`))
    (`KismetSystemLibrary.DrawDebugSphere` (`self.K2_GetActorLocation`) (`.SphereRadius` (`KismetSystemLibrary.GetComponentBounds` (`self.StaticMeshComponent`))) 12 (struct :`R` 0.03195 :`G` 1.0 :`A` 1.0) 0.25 1.0)))

(event `self.ReceiveTick`
  (params (DeltaSeconds :type "Float (single-precision)"))
  (bind (_outtransf_location _outtransf_rotation) (`KismetMathLibrary.BreakTransform` (`self.GetTargetTransform`)))
  (if (`self.bPickedUp`)
    (`self.K2_SetActorTransform` (`KismetMathLibrary.MakeTransform` _outtransf_location _outtransf_rotation))))

(fn `GetTargetTransform`
  (returns (OutTransf :type "Transform Structure"))
  (bind (_returnvalue_location _returnvalue_rotation) (`KismetMathLibrary.BreakTransform` (`self.GetTransform` (`GameplayStatics.GetPlayerCharacter` 0))))
  (return (`KismetMathLibrary.MakeTransform` (+ _returnvalue_location (* (`KismetMathLibrary.GetForwardVector` _returnvalue_rotation) (* (`.SphereRadius` (`KismetSystemLibrary.GetComponentBounds` (`self.StaticMeshComponent`))) 1.5))) _returnvalue_rotation)))

(fn `UserConstructionScript`
  (locals (ScaleOffset :type "Float (double-precision)" :default 0.0))
  (`parent.UserConstructionScript`)
  (set `self.ItemName` (`KismetStringLibrary.Conv_StringToName` (`KismetStringLibrary.LeftChop` (`KismetStringLibrary.RightChop` (`KismetSystemLibrary.GetClassDisplayName` (`GameplayStatics.GetObjectClass` self)) 3) 2))))